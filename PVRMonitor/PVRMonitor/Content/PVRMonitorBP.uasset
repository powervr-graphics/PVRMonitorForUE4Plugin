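; PVRMonitorBP bridges a PVRMonitorManager and an on-screen PVRMonitorUI widget for displaying performance-monitor counters.
; The construction script creates the manager; BeginPlay initializes it, then creates and shows the widget with a back-reference to this Blueprint, and EndPlay shuts the manager down.
; Wrapper functions expose manager pinging, counter lookup by name with a dummy fallback, name and bar-count queries, and counter group selection.
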(event EventBeginPlay
  (Class|PVRMonitorManager|InitializeManager (Variables|Default|GetPVRMonitorManagerVar))
  (CallFunction|InitializeUI)
  (Default|ShowUI (Variables|Default|GetPVRMonitorUI)))

(event EventEndPlay
  (params (EndPlayReason :type EEndPlayReason%20Enum :default "Destroyed"))
  (Class|PVRMonitorManager|DeInitializeManager (Variables|Default|GetPVRMonitorManagerVar)))

(fn ConstructionScript
  (bind _returnvalue (Game|ConstructObjectfromClass "/Script/PVRMonitorPlugin.PVRMonitorManager" self))
  (Variables|Default|SetPVRMonitorManagerVar _returnvalue))

(fn InitializeUI
  (bind _returnvalue (UserInterface|CreateWidget "/PVRMonitor/PVRMonitorUI.PVRMonitorUI_C"))
  (bind _output_get (Variables|Default|SetPVRMonitorUI _returnvalue))
  (Variables|/PVRMonitor/PVRMonitorUI.PVRMonitorUI_C|SetPVRMonitorBP _output_get self))

(fn GetCounterValues
  (params (Counter%20Name :type String))
  (bind _pvrmonitormanagervar (Variables|Default|GetPVRMonitorManagerVar))
  (bind _returnvalue (Class|PVRMonitorManager|GetCounterIndex _pvrmonitormanagervar Counter%20Name))
  (if (< _returnvalue 0)
    (return (Variables|Default|GetDummy))
    (else
      (bind _returnvalue_2 (Class|PVRMonitorManager|GetCounter _pvrmonitormanagervar _returnvalue))
      (return _returnvalue_2))))

(fn Update
  (Class|PVRMonitorManager|Ping (Variables|Default|GetPVRMonitorManagerVar)))

(fn GetCounterNames
  (bind _returnvalue (Class|PVRMonitorManager|GetCounterNames (Variables|Default|GetPVRMonitorManagerVar)))
  (return _returnvalue))

(fn GetNumBars
  (bind _returnvalue (Class|PVRMonitorManager|GetNumBars (Variables|Default|GetPVRMonitorManagerVar)))
  (return _returnvalue))

(fn GetCounterGroups
  (bind _returnvalue (Class|PVRMonitorManager|GetGroups (Variables|Default|GetPVRMonitorManagerVar)))
  (return _returnvalue))

(fn SetCounterGroup
  (params (Selected%20group :type Integer))
  (Class|PVRMonitorManager|SetGroup (Variables|Default|GetPVRMonitorManagerVar) Selected%20group))